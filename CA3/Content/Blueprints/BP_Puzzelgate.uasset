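; BP_Puzzelgate is a puzzle gate that swings open once enough items have been collected.
; A collect event increments the item count, and a separate check event compares it to the maximum.
; When the threshold is met, a DoOnce triggers the open event, where a timeline lerps the door's relative yaw to rotate it open a single time.
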(event Custom|open%20door
  (bind _door_rotation (Timeline|OpendoorAnim Play)
    (:Update
      (Transformation|SetRelativeRotation (Variables|Default|GetDoor) (Math|Rotator|MakeRotator 0.0 0.0 (Math|Float|Lerp 0.0 1.2e+02 _door_rotation)) false false))))

(event Custom|collect%20Item
  (Math|Integer|IncrementInt (Variables|Default|GetcurrentItemsCollected)))

(event Custom|oppendoorcheck
  (if (>= (Variables|Default|GetcurrentItemsCollected) (Variables|Default|GetmaxItemCollectable))
    (Utilities|FlowControl|DoOnce false
      (:Completed
        (CallFunction|OpenDoor)))))

(fn ConstructionScript)